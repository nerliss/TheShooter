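; Flamethrower weapon Blueprint that enables player input once attached to an actor and fires while the left mouse button is held, on a looping timer.
; Each shot sphere-traces forward from the muzzle along the camera's view, with debug drawing and hit-count printing.
; Hit first-person characters take random damage and catch fire; other hits spawn fire emitters.
; Emitter tracking and timed cleanup are disconnected, leaving DestroyFire's list unfilled here.
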(event `self.ReceiveTick`
  (params (DeltaSeconds :type "Float (single-precision)"))
  (`|ExecutionSequence`
    (:`then_0`
      (`/Engine/EditorBlueprintResources/StandardMacros.IsValid` (`self.GetAttachParentActor`)
        (:`Is Valid`
          (`/Engine/EditorBlueprintResources/StandardMacros.DoOnce` false
            (:`Completed`
              (`self.EnableInput` (`GameplayStatics.GetPlayerController` 0)))))))))

(event `Key|LeftMouseButton`
  (params (Key :type "Key Structure"))
  (:`Pressed`
    (`self.StartFire`)
    (bind _returnvalue (`KismetSystemLibrary.K2_SetTimerDelegate` (`|CreateDelegate` :!event `StartFire`) 0.2 true))
    (set `self.FiringTimerHandle` _returnvalue))
  (:`Released`
    (`KismetSystemLibrary.K2_ClearAndInvalidateTimerHandle` (`self.FiringTimerHandle`))))

(event `StartFire`
  (bind _returnvalue (`SceneComponent.GetSocketLocation` (`self.WeaponSkeletalMesh`) "MuzzleSocket"))
  (bind _returnvalue_2 (`SceneComponent.GetForwardVector` (`S_PlayerCharacter.CameraComp` (`self.PlayerRef`))))
  (bind (_outhits _returnvalue_3) (`KismetSystemLibrary.SphereTraceMulti` :`Start` (+ (* _returnvalue_2 50.0) _returnvalue) :`End` (+ _returnvalue (* _returnvalue_2 1200.0)) :`Radius` 15.0 :`TraceChannel` "TraceTypeQuery2" :`DrawDebugType` "ForDuration"))
  (if _returnvalue_3
    (`KismetSystemLibrary.PrintString` (`KismetStringLibrary.Conv_IntToString` (`KismetArrayLibrary.Array_Length` _outhits)))
    (for _array_element _outhits
      (`|ExecutionSequence`
        (:`then_0`
          (bind (_bblockinghit _binitialoverlap _time _distance _location _impactpoint _normal _impactnormal _physmat _hitactor) (`GameplayStatics.BreakHitResult` _array_element))
          (bind _asbp_first_person_character (cast `/Game/TheShooter/Core/Characters/BP_FirstPersonCharacter` _hitactor)
            (:`then`
              (`GameplayStatics.ApplyDamage` _asbp_first_person_character (`KismetMathLibrary.Conv_IntToDouble` (`KismetMathLibrary.Round` (`KismetMathLibrary.RandomFloatInRange` 4.0 10.0))) null (`self.PlayerRef`) "/Engine/EngineDamageTypes/DmgTypeBP_Environmental.DmgTypeBP_Environmental_C")
              (if (not (`/Game/TheShooter/Core/Characters/BP_FirstPersonCharacter.bIsOnFire` _asbp_first_person_character))
                (`/Game/TheShooter/Core/Characters/BP_FirstPersonCharacter.SetIsOnFire` _asbp_first_person_character)))
            (:`CastFailed`
              (bind _returnvalue_4 (`GameplayStatics.SpawnEmitterAtLocation` "/Game/StarterContent/Particles/P_Fire.P_Fire" _impactpoint)))))))))

(event `Destroy Fire`
  (for _array_element (`self.FireEmitters`)
    (set `self.bFistEligibleFound` true)
    (break))
  (if (`self.bFistEligibleFound`)
    (`ActorComponent.K2_DestroyComponent` _array_element)))

(fn `UserConstructionScript`)